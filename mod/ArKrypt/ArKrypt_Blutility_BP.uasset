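; Editor utility Blueprint that serves as a manual test harness for the ArKrypt_Functions encoding and encryption library.
; Each event runs one test on that class's default object: Base64, UTF-8, hex, int/byte conversion, ChaCha20 or JWT verification.
; Single tests process editable inputs, while multi tests round-trip preset or random data, some with expected-output, endianness or timing checks.
; Formatting helpers print results, mostly marked PASS/FAIL in multi tests, to the editor world.
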(event Custom|MultiTest_UTF8
  (MultiTests|MultiTestUTF8EncodeDecode))

(event Custom|MultiTest_HexToBytes
  (MultiTests|MultiTestHexHextoBytes))

(event Custom|MultiTest_ChaCha20
  (MultiTests|MultiTestChaCha20Func))

(event Custom|Test_ChaCha20_Decipher
  (SingleTests|SingleTestChaCha20Decipher))

(event Custom|MultiTest_BytesToInt
  (MultiTests|MultiTestIntBytestoInt))

(event Custom|MultiTest_Base64
  (MultiTests|MultiTestBase64EncodeDecode))

(event Custom|Test_ChaCha20_Cipher
  (SingleTests|SingleTestChaCha20Cipher))

(event Custom|Test_ChaCha20_KeyGen
  (SingleTests|SingleTestChaCha20KeyGen))

(event Custom|Test_ChaCha20_NonceGen
  (SingleTests|SingleTestChaCha20NonceGen))

(event Custom|Test_Verify_Base64_or_Hex
  (SingleTests|SingleTestVerifyBase64orHex))

(event Custom|Test_Verify_JWT
  (SingleTests|SingleTestVerifyJWT))

(event Custom|Test_Base64Encode
  (SingleTests|SingleTestBase64Encode))

(event Custom|Test_Base64Decode
  (SingleTests|SingleTestBase64Decode))

(fn SingleTestBase64Encode
  (bind _symcryptobj (Util|GetMyArKrypt))
  (bind _returnvalue (Default|StringtoBase64 _symcryptobj (Variables|Default|GetEncode_Input) (Variables|Default|GetbEncodeForURL)))
  (Util|MyLogF1 "ENCODE >>> {0}" _returnvalue))

(fn SingleTestBase64Decode
  (bind _symcryptobj (Util|GetMyArKrypt))
  (bind _returnvalue (Default|Base64toString _symcryptobj (Variables|Default|GetDecode_Input) (Variables|Default|GetbEncodeForURL)))
  (Util|MyLogF1 "DECODE >>> {0}" _returnvalue))

(fn MultiTestUTF8EncodeDecode
  (bind _returnvalue (Utilities|String|MakeLiteralString "0123456789ABCDEF"))
  (bind _l_failures (LocalVariables|GetL_FAILURES))
  (bind _symcryptobj (Util|GetMyArKrypt))
  (for (_array_element _array_index) (Variables|Default|GetMultiTest_Inputs)
    (bind _utf8bytes (Default|StringtoUTF8Bytes _symcryptobj _array_element))
    (LocalVariables|SetL_ByteDisp (Utilities|String|Append (Class|VictoryCore|GetNewlineCharacter) (Class|VictoryCore|InttoStringAscii 9)))
    (Utilities|Array|Clear (LocalVariables|GetL_Bytes4Test))
    (for (_array_element_2 _array_index_2) _utf8bytes
      (LocalVariables|SetL_ByteDisp (Util|MyFormatString "{0}{1} {2}" (Utilities|Array|MakeArray (LocalVariables|GetL_ByteDisp) (Utilities|String|Append (Utilities|String|GetSubstring _returnvalue (Math|Conversions|ToInteger(Byte) (/ _array_element_2 16))) (Utilities|String|GetSubstring _returnvalue (Math|Conversions|ToInteger(Byte) (Class|KismetMathLibrary|PercentByteByte _array_element_2 16)))) (Utilities|String|SelectString (Utilities|String|Append (Class|VictoryCore|GetNewlineCharacter) (Class|VictoryCore|InttoStringAscii 9)) "" (and (== (Math|Integer|%(Integer) (+ _array_index_2 1) 24) 0) (!= _array_index_2 (Utilities|Array|LastIndex _utf8bytes)))))))
      (Utilities|Array|Add (LocalVariables|GetL_Bytes4Test) (Utilities|String|Append (Utilities|String|GetSubstring _returnvalue (Math|Conversions|ToInteger(Byte) (/ _array_element_2 16))) (Utilities|String|GetSubstring _returnvalue (Math|Conversions|ToInteger(Byte) (Class|KismetMathLibrary|PercentByteByte _array_element_2 16))))))
    (Utilities|FlowControl|Sequence
      (:then_0
        (if (not (Utilities|Enum|Equal(Enum) (Utilities|String|JoinStringArray (LocalVariables|GetL_Bytes4Test) " ") (Utilities|Array|Get(acopy) (Variables|Default|GetMultiTest_UTF8_Expectations) _array_index)))
          (Utilities|Array|Add (LocalVariables|GetL_FAILURES) (Util|MyFormatString "FAILURE[{0}]: [{1}]" (Utilities|Array|MakeArray (Utilities|String|ToString(Integer) _array_index) (Utilities|Array|Get(acopy) (Variables|Default|GetMultiTest_UTF8_Expectations) _array_index))))))
      (:then_1
        (Util|MyLogF3 "UTF Test[{0}]: To UTF Bytes >>> [{1}]{2}" (Utilities|String|ToString(Integer) _array_index) _array_element (LocalVariables|GetL_ByteDisp)))
      (:then_2
        (bind _outstring (Default|UTF8BytestoString _symcryptobj _utf8bytes))
        (Util|MyLogF3 "UTF Test[{0}]: [{1}] To String >>> [{2}]" (Utilities|String|ToString(Integer) _array_index) (Utilities|String|SelectString "PASS" "FAIL" (Utilities|Enum|Equal(Enum) _array_element _outstring)) _outstring)
        (if (not (Utilities|Enum|Equal(Enum) _array_element _outstring))
          (Utilities|Array|Add (LocalVariables|GetL_FAILURES) (Util|MyFormatString "FAILURE[{0}]: [{1}] != [{2}]" (Utilities|Array|MakeArray (Utilities|String|ToString(Integer) _array_index) _outstring _array_element)))))))
  (if (Utilities|Array|IsValidIndex _l_failures)
    (for _array_element_3 _l_failures
      (Util|MyLog _array_element_3))
    (else
      (Util|MyLog "All UTF8 Tests Passed Successfully."))))

(fn MyFormatString
  (params (Format :type String) (Args :type Array%20of%20Strings))
  (Utilities|FlowControl|Sequence
    (:then_0
      (LocalVariables|SetL_Out Format)
      (for (_array_element _array_index) Args
        (LocalVariables|SetL_Out (Utilities|String|Replace (LocalVariables|GetL_Out) (Utilities|String|Append (Utilities|String|Append "{" (Utilities|String|ToString(Integer) _array_index)) "}") _array_element "CaseSensitive"))))
    (:then_1
      (return (LocalVariables|GetL_Out)))))

(fn MyLog
  (params (Log :type String))
  (bind _returnvalue (Class|PlacedEditorUtilityBase|GetEditorWorld))
  (Development|PrintString _returnvalue Log false))

(fn MyLogFormatted
  (params (LogFormat :type String) (Args :type Array%20of%20Strings))
  (Util|MyLog (Util|MyFormatString LogFormat Args)))

(fn MyLogF1
  (params (LogFormat :type String) (Arg0 :type String))
  (Util|MyLogFormatted LogFormat (Utilities|Array|MakeArray Arg0)))

(fn MyLogF2
  (params (LogFormat :type String) (Arg0 :type String) (Arg1 :type String))
  (Util|MyLogFormatted LogFormat (Utilities|Array|MakeArray Arg0 Arg1)))

(fn MyLogF3
  (params (LogFormat :type String) (Arg0 :type String) (Arg1 :type String) (Arg2 :type String))
  (Util|MyLogFormatted LogFormat (Utilities|Array|MakeArray Arg0 Arg1 Arg2)))

(fn GetMyArKrypt
  (bind _returnvalue (Class|VictoryCore|GetClassDefaultObject "/Game/Mods/ArKrypt/ArKrypt_Functions.ArKrypt_Functions_C"))
  (bind _asarkrypt_functions_c (Utilities|Casting|CastToArKrypt_Functions _returnvalue)
    (:then
      _)
    (:CastFailed
      _))
  (return _asarkrypt_functions_c))

(fn MultiTestBase64EncodeDecode
  (bind _bencodeforurl (Variables|Default|GetbEncodeForURL))
  (bind _l_failures (LocalVariables|GetL_FAILURES))
  (bind _symcryptobj (Util|GetMyArKrypt))
  (for (_array_element _array_index) (Variables|Default|GetMultiTest_Inputs)
    (Utilities|FlowControl|Sequence
      (:then_0
        (bind _returnvalue (Default|StringtoBase64 _symcryptobj _array_element _bencodeforurl))
        (Util|MyLogF2 "BASE64[{0}]: Encode >>> [{1}]" (Utilities|String|ToString(Integer) _array_index) _returnvalue))
      (:then_1
        (bind _returnvalue_2 (Default|Base64toString _symcryptobj _returnvalue _bencodeforurl))
        (Util|MyLogF3 "BASE64[{0}]: [{1}] Decode >>> [{2}]" (Utilities|String|ToString(Integer) _array_index) (Utilities|String|SelectString "PASS" "FAIL" (Utilities|Enum|Equal(Enum) _array_element _returnvalue_2)) _returnvalue_2)
        (if (not (Utilities|Enum|Equal(Enum) _array_element _returnvalue_2))
          (Utilities|Array|Add (LocalVariables|GetL_FAILURES) (Util|MyFormatString "FAILURE[{0}]: [{1}] != [{2}]" (Utilities|Array|MakeArray (Utilities|String|ToString(Integer) _array_index) _returnvalue_2 _array_element)))))))
  (if (Utilities|Array|IsValidIndex _l_failures)
    (for _array_element_2 _l_failures
      (Util|MyLog _array_element_2))
    (else
      (Util|MyLog "All BASE64 Tests Passed Successfully."))))

(fn MultiTestHexHextoBytes
  (bind _returnvalue (Utilities|String|MakeLiteralString "abc123 This Is Not Hex!"))
  (bind _symcryptobj (Util|GetMyArKrypt))
  (for _index (range 0 3)
    (Utilities|FlowControl|Sequence
      (:then_0
        (bind _returnvalue_2 (Default|RandomBytes _symcryptobj (Math|Random|RandomIntegerinRange 7 43) false))
        (bind _hex (Default|BytestoHex _symcryptobj _returnvalue_2))
        (Util|MyLogF1 "Initial Hex  >>> [{0}]" _hex))
      (:then_1
        (bind _returnvalue_3 (Default|HextoBytes _symcryptobj _hex))
        (bind _hex_2 (Default|BytestoHex _symcryptobj _returnvalue_3))
        (Util|MyLogF2 "ToBytesToHex >>> [{0}] [{1}]" _hex_2 (Utilities|String|SelectString "PASS" "FAIL" (Utilities|Enum|Equal(Enum) _hex _hex_2))))
      (:then_2
        (Util|MyLogF1 "ToUpperInput >>> [{0}]" (Class|KismetStringLibrary|ToUpper _hex))
        (bind _returnvalue_4 (Default|HextoBytes _symcryptobj (Class|KismetStringLibrary|ToUpper _hex)))
        (bind _hex_3 (Default|BytestoHex _symcryptobj _returnvalue_4))
        (Util|MyLogF2 "ToUpperToHex >>> [{0}] [{1}]" _hex_3 (Utilities|String|SelectString "PASS" "FAIL" (Utilities|Enum|Equal(Enum) _hex _hex_3))))
      (:then_3
        (Util|MyLogF1 "UnevenInput  >>> [{0}]" (Utilities|String|GetSubstring _hex 1 (- (Utilities|String|Len _hex) 1)))
        (bind _returnvalue_5 (Default|HextoBytes _symcryptobj (Utilities|String|GetSubstring _hex 1 (- (Utilities|String|Len _hex) 1))))
        (bind _hex_4 (Default|BytestoHex _symcryptobj _returnvalue_5))
        (Util|MyLogF2 "UnevenOutput >>> [{0}] [{1}]" _hex_4 (Utilities|String|SelectString "PASS" "FAIL" (Utilities|Enum|Equal(Enum) (Utilities|String|Append "0" (Utilities|String|GetSubstring _hex 1 (- (Utilities|String|Len _hex) 1))) _hex_4))))))
  (bind _returnvalue_6 (Default|HextoBytes _symcryptobj _returnvalue))
  (Util|MyLogF3 "BadInput     >>> [{0}] ResultByteLen [{1}] [{2}]" _returnvalue (Utilities|String|ToString(Integer) (Utilities|Array|Length _returnvalue_6)) (Utilities|String|SelectString "PASS" "FAIL" (== (Utilities|Array|Length _returnvalue_6) 0))))

(fn ByteBinaryDisplay
  (params (Input :type Byte))
  (Utilities|FlowControl|Sequence
    (:then_0
      (for _index (range 0 7)
        (LocalVariables|SetL_Binary (Utilities|String|Append (LocalVariables|GetL_Binary) (Utilities|String|SelectString "1" "0" (== (Class|KismetMathLibrary|AndIntInt (Math|Conversions|ToInteger(Byte) Input) (Class|KismetMathLibrary|MultiplyMultiplyIntInt 2 (- (Class|KismetSystemLibrary|MakeLiteralInteger 7) _index))) (Class|KismetMathLibrary|MultiplyMultiplyIntInt 2 (- (Class|KismetSystemLibrary|MakeLiteralInteger 7) _index))))))))
    (:then_1
      (return (LocalVariables|GetL_Binary)))))

(fn MultiTestIntBytestoInt
  (bind _returnvalue (Class|KismetSystemLibrary|MakeLiteralInteger 2147483647))
  (bind _returnvalue_2 (Math|Random|RandomIntegerinRange 1 2147483647))
  (bind _symcryptobj (Util|GetMyArKrypt))
  (for _index (range 0 3)
    (Utilities|FlowControl|Sequence
      (:then_0
        (LocalVariables|SetL_TestInteger (Math|Integer|SelectInt _returnvalue_2 (- (* _returnvalue_2 -1) 1) (Math|Random|RandomBool))))
      (:then_1
        (for _index_2 (range 0 1)
          (Utilities|FlowControl|Sequence
            (:then_0
              (bind _returnvalue_3 (Default|InttoBytes _symcryptobj (LocalVariables|GetL_TestInteger) (Math|Conversions|ToBoolean(Integer) _index_2)))
              (LocalVariables|SetL_ByteDisp (Util|MyFormatString "{0} {1} {2} {3}" (Utilities|Array|MakeArray (Util|ByteBinaryDisplay (Utilities|Array|Get(acopy) _returnvalue_3)) (Util|ByteBinaryDisplay (Utilities|Array|Get(acopy) _returnvalue_3 1)) (Util|ByteBinaryDisplay (Utilities|Array|Get(acopy) _returnvalue_3 2)) (Util|ByteBinaryDisplay (Utilities|Array|Get(acopy) _returnvalue_3 3)))))
              (Util|MyLogF3 "INT 2 BYTES >>> [{0}] [{1}] -> [{2}]" (Utilities|String|SelectString "LE" "BE" (Math|Conversions|ToBoolean(Integer) _index_2)) (Utilities|String|ToString(Integer) (LocalVariables|GetL_TestInteger)) (LocalVariables|GetL_ByteDisp)))
            (:then_1
              (bind _returnvalue_4 (Default|BytestoInt _symcryptobj _returnvalue_3 (Math|Conversions|ToBoolean(Integer) _index_2)))
              (Util|MyLogF4 "BYTES 2 INT >>> [{0}] [{1}] -> [{2}] [{3}]" (Utilities|String|SelectString "LE" "BE" (Math|Conversions|ToBoolean(Integer) _index_2)) (LocalVariables|GetL_ByteDisp) (Utilities|String|ToString(Integer) _returnvalue_4) (Utilities|String|SelectString "PASS" "FAIL" (== (LocalVariables|GetL_TestInteger) _returnvalue_4))))
            (:then_2
              (bind _returnvalue_5 (Default|InttoBytes _symcryptobj (LocalVariables|GetL_TestInteger) (not (Math|Conversions|ToBoolean(Integer) _index_2))))
              (Util|MyLogF4 "REVERSE BYTES > [{0}] [{1}] -> [{2}] [{3}]" (Utilities|String|SelectString "LE" "BE" (Math|Conversions|ToBoolean(Integer) _index_2)) (LocalVariables|GetL_ByteDisp) (Util|MyFormatString "{0} {1} {2} {3}" (Utilities|Array|MakeArray (Util|ByteBinaryDisplay (Utilities|Array|Get(acopy) _returnvalue_5)) (Util|ByteBinaryDisplay (Utilities|Array|Get(acopy) _returnvalue_5 1)) (Util|ByteBinaryDisplay (Utilities|Array|Get(acopy) _returnvalue_5 2)) (Util|ByteBinaryDisplay (Utilities|Array|Get(acopy) _returnvalue_5 3)))) (Utilities|String|SelectString "PASS" "FAIL" (Math|Boolean|ANDBoolean (== (Utilities|Array|Get(acopy) _returnvalue_3) (Utilities|Array|Get(acopy) _returnvalue_5 3)) (== (Utilities|Array|Get(acopy) _returnvalue_3 1) (Utilities|Array|Get(acopy) _returnvalue_5 2)) (== (Utilities|Array|Get(acopy) _returnvalue_3 2) (Utilities|Array|Get(acopy) _returnvalue_5 1)) (== (Utilities|Array|Get(acopy) _returnvalue_3 3) (Utilities|Array|Get(acopy) _returnvalue_5)))))))))))
  (for _index_3 (range 0 11)
    (LocalVariables|SetL_Ran (Math|Random|RandomIntegerinRange 1 2147483647))
    (LocalVariables|SetL_TestInteger (+ _returnvalue (LocalVariables|GetL_Ran)))
    (Utilities|FlowControl|Sequence
      (:then_0
        (Util|MyLogF3 "ROLLOVER ADD >>  [{0}] + [{1}] = [{2}]" (Class|KismetStringLibrary|LeftPad (Utilities|String|ToString(Integer) _returnvalue) 11) (Class|KismetStringLibrary|LeftPad (Utilities|String|ToString(Integer) (LocalVariables|GetL_Ran)) 11) (Class|KismetStringLibrary|LeftPad (Utilities|String|ToString(Integer) (LocalVariables|GetL_TestInteger)) 11)))
      (:then_1
        (for _index_4 (range 0 1)
          (Utilities|FlowControl|Sequence
            (:then_0
              (bind _returnvalue_6 (Default|InttoBytes _symcryptobj (LocalVariables|GetL_TestInteger) (Math|Conversions|ToBoolean(Integer) _index_4)))
              (LocalVariables|SetL_ByteDisp (Util|MyFormatString "{0} {1} {2} {3}" (Utilities|Array|MakeArray (Util|ByteBinaryDisplay (Utilities|Array|Get(acopy) _returnvalue_6)) (Util|ByteBinaryDisplay (Utilities|Array|Get(acopy) _returnvalue_6 1)) (Util|ByteBinaryDisplay (Utilities|Array|Get(acopy) _returnvalue_6 2)) (Util|ByteBinaryDisplay (Utilities|Array|Get(acopy) _returnvalue_6 3)))))
              (Util|MyLogF3 "INT 2 BYTES >>> [{0}] [{1}] -> [{2}]" (Utilities|String|SelectString "LE" "BE" (Math|Conversions|ToBoolean(Integer) _index_4)) (Utilities|String|ToString(Integer) (LocalVariables|GetL_TestInteger)) (LocalVariables|GetL_ByteDisp)))
            (:then_1
              (bind _returnvalue_7 (Default|BytestoInt _symcryptobj _returnvalue_6 (Math|Conversions|ToBoolean(Integer) _index_4)))
              (Util|MyLogF4 "BYTES 2 INT >>> [{0}] [{1}] -> [{2}] [{3}]" (Utilities|String|SelectString "LE" "BE" (Math|Conversions|ToBoolean(Integer) _index_4)) (LocalVariables|GetL_ByteDisp) (Utilities|String|ToString(Integer) _returnvalue_7) (Utilities|String|SelectString "PASS" "FAIL" (== (LocalVariables|GetL_TestInteger) _returnvalue_7))))
            (:then_2
              (bind _returnvalue_8 (Default|InttoBytes _symcryptobj (LocalVariables|GetL_TestInteger) (not (Math|Conversions|ToBoolean(Integer) _index_4))))
              (Util|MyLogF4 "REVERSE BYTES > [{0}] [{1}] -> [{2}] [{3}]" (Utilities|String|SelectString "LE" "BE" (Math|Conversions|ToBoolean(Integer) _index_4)) (LocalVariables|GetL_ByteDisp) (Util|MyFormatString "{0} {1} {2} {3}" (Utilities|Array|MakeArray (Util|ByteBinaryDisplay (Utilities|Array|Get(acopy) _returnvalue_8)) (Util|ByteBinaryDisplay (Utilities|Array|Get(acopy) _returnvalue_8 1)) (Util|ByteBinaryDisplay (Utilities|Array|Get(acopy) _returnvalue_8 2)) (Util|ByteBinaryDisplay (Utilities|Array|Get(acopy) _returnvalue_8 3)))) (Utilities|String|SelectString "PASS" "FAIL" (Math|Boolean|ANDBoolean (== (Utilities|Array|Get(acopy) _returnvalue_6) (Utilities|Array|Get(acopy) _returnvalue_8 3)) (== (Utilities|Array|Get(acopy) _returnvalue_6 1) (Utilities|Array|Get(acopy) _returnvalue_8 2)) (== (Utilities|Array|Get(acopy) _returnvalue_6 2) (Utilities|Array|Get(acopy) _returnvalue_8 1)) (== (Utilities|Array|Get(acopy) _returnvalue_6 3) (Utilities|Array|Get(acopy) _returnvalue_8))))))))))))

(fn MyLogF4
  (params (LogFormat :type String) (Arg0 :type String) (Arg1 :type String) (Arg2 :type String) (Arg3 :type String))
  (Util|MyLogFormatted LogFormat (Utilities|Array|MakeArray Arg0 Arg1 Arg2 Arg3)))

(fn SingleTestChaCha20Cipher
  (bind _symcryptobj (Util|GetMyArKrypt))
  (bind (_ciphertext _bsuccess _error) (Default|ChaCha20CipherString _symcryptobj (Variables|Default|GetChaCha20_Cipher_Plaintext) (Variables|Default|GetChaCha20_Key) (Variables|Default|GetChaCha20_Nonce/IV) (Variables|Default|GetbChaCha20_UseBase64) (Variables|Default|GetChaCha20_InitialCounter)))
  (if _bsuccess
    (Util|MyLogF1 "ChaCha20 Cipher >>> {0}" _ciphertext)
    (else
      (Util|MyLogF2 "ChaCha20 Cipher >>> FAILED! CipherText [{0}] Error [{1}]" _ciphertext _error))))

(fn SingleTestChaCha20KeyGen
  (bind _bchacha20_usebase64 (Variables|Default|GetbChaCha20_UseBase64))
  (bind _symcryptobj (Util|GetMyArKrypt))
  (bind _newkey (Default|ChaCha20KeyGen _symcryptobj _bchacha20_usebase64))
  (Util|MyLogF2 "ChaCha20 KeyGen [{0}] >>> {1}" (Utilities|String|SelectString "B64" "HEX" _bchacha20_usebase64) _newkey))

(fn SingleTestChaCha20NonceGen
  (bind _bchacha20_usebase64 (Variables|Default|GetbChaCha20_UseBase64))
  (bind _symcryptobj (Util|GetMyArKrypt))
  (bind _nonce (Default|ChaCha20NonceGen _symcryptobj _bchacha20_usebase64))
  (Util|MyLogF2 "ChaCha20 NonceGen [{0}] >>> {1}" (Utilities|String|SelectString "B64" "HEX" _bchacha20_usebase64) _nonce))

(fn SingleTestChaCha20Decipher
  (bind _symcryptobj (Util|GetMyArKrypt))
  (bind (_plaintext _bsuccess _error) (Default|ChaCha20DecipherString _symcryptobj (Variables|Default|GetChaCha20_Cipher_CipherText) (Variables|Default|GetChaCha20_Key) (Variables|Default|GetChaCha20_Nonce/IV) (Variables|Default|GetbChaCha20_UseBase64) (Variables|Default|GetChaCha20_InitialCounter)))
  (if _bsuccess
    (Util|MyLogF1 "ChaCha20 Decipher >>> {0}" _plaintext)
    (else
      (Util|MyLogF2 "ChaCha20 Decipher >>> FAILED! PlainText [{0}] Error [{1}]" _plaintext _error))))

(fn MultiTestChaCha20Func
  (bind _returnvalue (Class|VictoryCore|GetRealWorldUtcTimeinSeconds))
  (Utilities|FlowControl|Sequence
    (:then_0
      (LocalVariables|SetbL_Base64 true))
    (:then_1
      (LocalVariables|SetbL_Base64 false)))
  (Utilities|Array|Clear (LocalVariables|GetL_Results))
  (Utilities|FlowControl|Sequence
    (:then_0
      (LocalVariables|SetL_TestStarted _returnvalue))
    (:then_1
      (bind _symcryptobj (Util|GetMyArKrypt))
      (bind _newkey (Default|ChaCha20KeyGen _symcryptobj (LocalVariables|GetbL_Base64)))
      (bind _nonce (Default|ChaCha20NonceGen _symcryptobj (LocalVariables|GetbL_Base64))))
    (:then_2
      (for (_array_element _array_index) (Variables|Default|GetMultiTest_Inputs)
        (bind (_ciphertext _bsuccess) (Default|ChaCha20CipherString _symcryptobj _array_element _newkey _nonce (LocalVariables|GetbL_Base64) 1))
        (if _bsuccess
          (bind _plaintext (Default|ChaCha20DecipherString _symcryptobj _ciphertext _newkey _nonce (LocalVariables|GetbL_Base64) 1)))
        (Utilities|Array|Add (LocalVariables|GetL_Results) (Util|MyFormatString "ChaCha20 [{5}] [{0}]: [{1}] [{2}] >>> [{3}] >>> [{4}]" (Utilities|Array|MakeArray (Utilities|String|ToString(Integer) _array_index) (Utilities|String|SelectString "PASS" "FAIL!!!" (Utilities|Enum|Equal(Enum) _plaintext _array_element)) _array_element _ciphertext _plaintext (Utilities|String|SelectString "B64" "HEX" (LocalVariables|GetbL_Base64))))))
      (LocalVariables|SetL_TestEnded _returnvalue)
      (Util|MyLogF3 "ChaCha20 MultiTest [{0}] Key [{1}] Nonce [{2}]" (Utilities|String|SelectString "B64" "HEX" (LocalVariables|GetbL_Base64)) _newkey _nonce)
      (for _array_element_2 (LocalVariables|GetL_Results)
        (Util|MyLog _array_element_2))
      (Util|MyLogF2 "ChaCha20 MultiTest [{0}] Time [{1}]" (Utilities|String|SelectString "B64" "HEX" (LocalVariables|GetbL_Base64)) (Utilities|String|ToString(Float) (- (LocalVariables|GetL_TestEnded) (LocalVariables|GetL_TestStarted)))))))

(fn SingleTestVerifyBase64orHex
  (bind _test_verifyinput (Variables|Default|GetTest_VerifyInput))
  (bind _symcryptobj (Util|GetMyArKrypt))
  (Utilities|FlowControl|Sequence
    (:then_0
      (bind _bverified (Default|VerifyBase64 _symcryptobj _test_verifyinput (Variables|Default|GetbEncodeForURL)))
      (Util|MyLogF2 "[{0}] {1}" _test_verifyinput (Utilities|String|SelectString "VALID BASE64" "NOT VALID BASE64" _bverified)))
    (:then_1
      (bind _bverified_2 (Default|VerifyHex _symcryptobj _test_verifyinput))
      (Util|MyLogF2 "[{0}] {1}" _test_verifyinput (Utilities|String|SelectString "VALID HEX" "NOT VALID HEX" _bverified_2)))))

(fn SingleTestVerifyJWT
  (bind _jwt_input (Variables|Default|GetJWT_Input))
  (bind _bjwt_noparse (Variables|Default|GetbJWT_NoParse))
  (bind _symcryptobj (Util|GetMyArKrypt))
  (Util|MyLogF2 "VerifyJWT - NoParse? [{0}] - [{1}]" (Utilities|String|ToString(Boolean) _bjwt_noparse) _jwt_input)
  (bind (_bverified _header _data _signature) (Default|VerifyJWT _symcryptobj _jwt_input _bjwt_noparse))
  (Util|MyLogFormatted "VerifyJWT - {1} {0}Header [{2}] {0}Data [{3}] {0}Signature [{4}]" (Utilities|Array|MakeArray (Class|VictoryCore|GetNewlineCharacter) (Utilities|String|SelectString "VALID JWT" "NOT VALID JWT!!!" _bverified) _header _data _signature)))